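; Enemy Blueprint that handles health bar and floating hit-number UI over a C++ parent class.
; BeginPlay links the health bar widget to this enemy and hides it; show and hide events toggle it, with show also calling the parent C++ implementation.
; Hit events spawn an animated number widget at the projected screen position of the hit, carrying damage and headshot flag, then register it with its world location through StoreHitNumber.
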(event `self.ReceiveBeginPlay`
  (bind _asenemy_healthbar_bp (cast `/Game/_Game/HUD/EnemyHealthbarBp` (`WidgetComponent.GetUserWidgetObject` (`self.HealthBar`))))
  (set `/Game/_Game/HUD/EnemyHealthbarBp.Enemy` self _asenemy_healthbar_bp)
  (`Widget.SetVisibility` (`WidgetComponent.GetUserWidgetObject` (`self.HealthBar`)) "Hidden"))

(event `self.ShowHealthBar`
  (`Widget.SetVisibility` (`WidgetComponent.GetUserWidgetObject` (`self.HealthBar`)) "Visible")
  ;[1 1 1 1 14] Ruft den C++ code auf
  (`parent.ShowHealthBar`))

(event `self.HideHealthBar`
  (`Widget.SetVisibility` (`WidgetComponent.GetUserWidgetObject` (`self.HealthBar`)) "Hidden"))

(event `self.ShowHitNumer`
  (params (Damage :type Integer) (HitLocation :type "Vector Structure") (HeadShot :type Boolean))
  (bind _returnvalue (`|CreateWidget` "/Game/_Game/HUD/HitNumber.HitNumber_C"))
  (`UserWidget.AddToViewport` _returnvalue 0)
  (`UserWidget.SetPositionInViewport` _returnvalue (`GameplayStatics.ProjectWorldToScreen` (`GameplayStatics.GetPlayerController` 0) HitLocation) true)
  (`self.StoreHitNumber` _returnvalue HitLocation)
  (set `/Game/_Game/HUD/HitNumber.HitText` (`KismetTextLibrary.Conv_IntToText` Damage) _returnvalue)
  (set `/Game/_Game/HUD/HitNumber.IsHeadShot` HeadShot _returnvalue)
  (`UserWidget.PlayAnimation` _returnvalue (`/Game/_Game/HUD/HitNumber.HitNumberAnimation` _returnvalue) 0.0 1 "Forward" 1.0 false))

(fn `UserConstructionScript`)