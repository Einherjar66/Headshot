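; Health pickup actor that applies HealingAmount to a ShooterCharacter_BP entering its Sphere overlap.
; The overlap handler adds the amount to Health, but sets Health to zero, not MaxHealth, when the sum would exceed MaxHealth.
; It then plays HealthPickupSound at the pickup's location and destroys itself.
; Other overlapping actors are ignored through the failed cast.
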(event `self.Sphere.OnComponentBeginOverlap`
  (params (OverlappedComponent :type "PrimitiveComponent Object Reference") (OtherActor :type "Actor Object Reference") (OtherComp :type "PrimitiveComponent Object Reference") (OtherBodyIndex :type Integer) (bFromSweep :type Boolean) (SweepResult :type "HitResult Structure (by ref)"))
  (bind _asshooter_character_bp (cast `/Game/_Game/Character/ShooterCharacter_BP` OtherActor))
  (bind _returnvalue (+ (`ShooterCharacter.Health` _asshooter_character_bp) (`self.HealingAmount`)))
  (if (> _returnvalue (`ShooterCharacter.MaxHealth` _asshooter_character_bp))
    (set `ShooterCharacter.Health` 0.0 _asshooter_character_bp)
    (else
      (set `ShooterCharacter.Health` _returnvalue _asshooter_character_bp)))
  (`GameplayStatics.PlaySoundAtLocation` (`self.HealthPickupSound`) (`self.K2_GetActorLocation`) (struct) 1.0 1.0 0.0 null null null)
  (`self.K2_DestroyActor`))

(fn `UserConstructionScript`)